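; BP_ShootingCharacter_Tester is a shooting-game character Blueprint that, judging by its name, serves as a test bed for input and movement.
; Pressing 1 runs a short forward line trace with debug drawing; a hit switches movement to Flying, then back to Walking after a delay.
; Enhanced Input plays a single-shot rifle montage on shoot and sets IsCrouch on crouch start, clearing it only on the action's Canceled event.
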(event EventBeginPlay)

(event Collision|EventActorBeginOverlap
  (params (OtherActor :type Actor%20Object%20Reference)))

(event EventTick
  (params (DeltaSeconds :type Float%20%28single-precision%29)))

(event Input|KeyboardEvents|1
  (params (Key :type Key%20Structure :default "None"))
  (bind _self self)
  (bind _returnvalue (Transformation|GetActorLocation _self))
  (:Pressed
    (bind _returnvalue_2 (Collision|LineTraceByChannel _returnvalue (+ _returnvalue (* (Transformation|GetActorForwardVector _self) 1e+02)) "TraceTypeQuery1" false 0 "ForDuration"))
    (if _returnvalue_2
      (Pawn|Components|CharacterMovement|SetMovementMode (Variables|Character|GetCharacterMovement) "MOVE_Flying" 0)
      (Utilities|FlowControl|Delay 4.0)
      (Pawn|Components|CharacterMovement|SetMovementMode (Variables|Character|GetCharacterMovement) "MOVE_Walking" 0))))

(event Input|EnhancedActionEvents|EnhancedInputActionIA_Shoot
  (params (ActionValue :type Boolean) (ElapsedSeconds :type Float%20%28double-precision%29) (TriggeredSeconds :type Float%20%28double-precision%29) (InputAction :type Input%20Action%20Object%20Reference :default "/Game/ThirdPerson/Input/Actions/IA_Shoot.IA_Shoot"))
  (:Started
    (Animation|PlayAnimMontage "/Game/Characters/Mannequins/Animations/InPlace/Rifle_ShootOnce_Montage.Rifle_ShootOnce_Montage" 1.0 "None")))

(event Input|EnhancedActionEvents|EnhancedInputActionIA_Crouch
  (params (ActionValue :type Boolean) (ElapsedSeconds :type Float%20%28double-precision%29) (TriggeredSeconds :type Float%20%28double-precision%29) (InputAction :type Input%20Action%20Object%20Reference :default "/Game/ThirdPerson/Input/Actions/IA_Crouch.IA_Crouch"))
  (:Started
    (Variables|Default|SetbIsCrouch true))
  (:Canceled
    (Variables|Default|SetbIsCrouch false)))

(fn ConstructionScript)